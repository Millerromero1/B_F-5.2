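; Enemy AI character that roams randomly, chases seen pawns and fires a rifle at them.
; A short timed loop restarts roaming and clears the sighting flag, while Vision sightings trigger a move-to that fires on arrival.
; Shots play a montage with effects and apply line-trace damage along the mesh's right vector.
; Death ragdolls it, credits a player kill and destroys it; Tick updates a camera-facing health bar.
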(event OnSeePawn(Vision)
  (params (Pawn :type Pawn%20Object%20Reference))
  (CallFunction|ChaseTarget Pawn)
  (Variables|Default|Setseetarget? true))

(event Custom|Serch%20Around
  ;[0 0 0] Around
  (if (not (Variables|Default|Getseetarget?))
    (AI|AIMoveTo self (.RandomLocation (AI|Navigation|GetRandomReachablePointinRadius (Transformation|GetActorLocation) 2e+03 0 0)) 0 3e+02 false
      (:OnSuccess
        (Utilities|FlowControl|Delay 1.0)
        (CallFunction|SerchAround)))))

(event Custom|Chase%20target
  (params (TargetActor :type Actor%20Object%20Reference))
  (AI|AIMoveTo self "0, 0, 0" TargetActor 4.5e+02 false
    (:OnSuccess
      (CallFunction|Shoot TargetActor))))

(event Custom|Shoot
  (params (Target%20actor :type Actor%20Object%20Reference))
  (bind _mesh (Variables|Character|GetMesh))
  (bind _ak (Variables|Default|GetAK))
  (bind _returnvalue (Transformation|GetSocketTransform _ak "b_gun_muzzleflash" "RTS_World"))
  (bind _returnvalue_2 (Transformation|GetWorldRotation _mesh))
  (if (not (Variables|Default|GetIsdaed?))
    (Pawn|SetControlRotation (Pawn|GetController) (Math|Rotator|FindLookatRotation (Transformation|GetActorLocation) (Transformation|GetActorLocation Target%20actor)))
    (Animation|Montage|PlayMontage (Variables|Character|GetMesh) "/Game/S_anim/Fire_Rifle_Ironsights_Montage.Fire_Rifle_Ironsights_Montage"
      (:then
        (Effects|SpawnEmitterAttached "/Game/InfinityBladeEffects/Effects/FX_Monsters/FX_Monster_Gruntling/Master/P_BackPack_MuzzleFlash.P_BackPack_MuzzleFlash" (Variables|Default|GetAK) "b_gun_muzzleflash" (.location _returnvalue) _returnvalue_2 "0.100000,0.100000,0.100000" "KeepWorldPosition" true "AutoRelease")
        (Audio|PlaySoundatLocation "/Game/Sound/MS_rifle.MS_rifle" (Transformation|GetActorLocation) "0, 0, 0" 1.0 1.0 0.0 0 0 0 0)
        (bind (_outhit _returnvalue_3) (Collision|LineTraceByChannel (.location _returnvalue) (+ (.location _returnvalue) (* (Math|Vector|GetRightVector _returnvalue_2) 3e+03)) "TraceTypeQuery1" false 0 "None"))
        (if _returnvalue_3
          (Game|Damage|ApplyDamage (.HitActor (Collision|BreakHitResult _outhit)) 2.0 0 0)
          (Effects|SpawnEmitteratLocation "/Game/InfinityBladeEffects/Effects/FX_Monsters/FX_Monster_Troll/death/P_TrollDeathImpact.P_TrollDeathImpact" (.ImpactPoint (Collision|BreakHitResult _outhit)) (Math|Rotator|MakeRotfromX (.Normal (Collision|BreakHitResult _outhit))) "0.700000,0.700000,0.700000"))))))

(event EventBeginPlay
  (CallFunction|SerchAround)
  (Utilities|FlowControl|Delay 0.32 :!label _label)
  (CallFunction|SerchAround)
  (Variables|Default|Setseetarget? false)
  (goto _label))

(event EventTick
  (params (DeltaSeconds :type Float%20%28single-precision%29))
  (bind _aswb_e_h (Utilities|Casting|CastToWB_E_H (UserInterface|GetWidget (Variables|Default|GetHeatlh%20bar))))
  (Progress|SetPercent (Variables|/Game/WB_E_H.WB_E_H_C|GetHealthbar _aswb_e_h) (/ (Variables|Default|GetHealth) 2e+01))
  (Transformation|SetWorldRotation (Variables|Default|GetHeatlh%20bar) (Math|Rotator|FindLookatRotation (Transformation|GetActorLocation) (Transformation|GetActorLocation (Game|GetPlayerCameraManager 0))) false false))

(event Game|Damage|EventAnyDamage
  (params (Damage :type Float%20%28single-precision%29) (DamageType :type Damage%20Type%20Object%20Reference) (InstigatedBy :type Controller%20Object%20Reference) (DamageCauser :type Actor%20Object%20Reference))
  ;[1 1 1] healjt
  (bind _output_get (Variables|Default|SetHealth (- (Variables|Default|GetHealth) Damage)))
  (if (<= _output_get 0.0)
    (Physics|SetSimulatePhysics (Variables|Character|GetMesh) true)
    (Pawn|Components|CharacterMovement|SetMovementMode (Variables|Character|GetCharacterMovement) "MOVE_None" 0)
    (Variables|Default|SetIsdaed? true)
    (Rendering|SetVisibility (Variables|Default|GetHeatlh%20bar) false false)
    (Collision|SetCollisionEnabled (Variables|Collision|GetCapsuleComponent) "PhysicsOnly")
    (bind _asbp_third_person_character (Utilities|Casting|CastToBP_ThirdPersonCharacter (Game|GetPlayerCharacter 0)))
    (Variables|/Game/ThirdPerson/Blueprints/BP_ThirdPersonCharacter.BP_ThirdPersonCharacter_C|Setkills _asbp_third_person_character (+ (Variables|/Game/ThirdPerson/Blueprints/BP_ThirdPersonCharacter.BP_ThirdPersonCharacter_C|Getkills _asbp_third_person_character) 1))
    (Utilities|FlowControl|Delay 1.5)
    (Actor|DestroyActor)))

(fn ConstructionScript)